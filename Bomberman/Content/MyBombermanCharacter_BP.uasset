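; Player character Blueprint for a Bomberman-style game that handles movement and bomb placement.
; MoveForward and MoveRight axes add movement input along fixed world Y and negative X axes, independent of control rotation.
; PlaceBomb spawns a Bomb through SpawnNewActor.CreateActor just ahead of the capsule at a fixed world height, using the character's rotation.
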(event `InputAxis|MoveForward`
  (params (AxisValue :type "Float (single-precision)"))
  (`self.AddMovementInput` (0.0 2.0 0.0) AxisValue))

(event `InputAxis|MoveRight`
  (params (AxisValue :type "Float (single-precision)"))
  (`self.AddMovementInput` (-2.0 0.0 0.0) AxisValue))

(event `InputAction|PlaceBomb`
  (params (Key :type "Key Structure"))
  (:`Pressed`
    (`SpawnNewActor.CreateActor` (`self.SpawnNewActor`) "/Script/Bomberman.Bomb" (+ (* (`self.K2_GetActorLocation`) (1.0 1.0 0.0)) (* (`SceneComponent.GetForwardVector` (`self.CapsuleComponent`)) (100.0 100.0 0.0)) (0.0 0.0 21.0)) (`self.K2_GetActorRotation`))))

(fn `UserConstructionScript`)